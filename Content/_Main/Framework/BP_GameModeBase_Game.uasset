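; Game mode that starts a match from the lobby and runs turn order for color-keyed players.
; SetTurn cycles to the next color held by a player, wrapping around, then updates turn flags in the GameState's player map and widget data.
; After a short delay, it refreshes every player's game UI and shows the turn UI to the active player.
; Player controllers are reached through each PlayerState, looked up by unique net ID.
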(event `StartNewGame`
  ;[1 1 1] Start New game from Lobby
  (bind _gamestate (message `/Game/_Main/Blueprints/Interfaces/BPI_GameState.GetGameState` (`GameplayStatics.GetGameState`)))
  (`/Game/_Main/Framework/BP_GameStateBase_Game.SetPlayerInfo` _gamestate)
  (`self.SetTurn`)
  (`self.CreateWidgetsForPlayers`))

(event `SetTurn`
  ;[1 1 1] Set Current Turn to the next player
  (bind _nextcolor (`self.Select Next Color`))
  (bind _playerid (`self.UpdatePlayerTurn` _nextcolor))
  (`KismetSystemLibrary.Delay` 0.2)
  (`self.CreatePlayersListWidget`)
  (`self.ShowNextPlayerUI` _playerid))

(fn `CreatePlayersListWidget`
  (bind _gamestate (message `/Game/_Main/Blueprints/Interfaces/BPI_GameState.GetGameState` (`GameplayStatics.GetGameState`)))
  (bind _players (`/Game/_Main/Framework/BP_GameStateBase_Game.Players` _gamestate))
  (bind _keys (`BlueprintMapLibrary.Map_Keys` _players))
  (for _array_element _keys
    (bind _playercontroller (message `/Game/_Main/Blueprints/Interfaces/BPI_CharacterController.GetPlayerController` (`PlayerState.GetPlayerController` (`GameplayStatics.GetPlayerStateFromUniqueNetId` (`.PlayerUniqueId_13_A48F12A04FD4F1A5D458D2B63D7A2242` (break `/Game/_Main/Blueprints/Structures/S_PlayerInfo` (`BlueprintMapLibrary.Map_Find` _players _array_element)))))))
    (`/Game/_Main/Framework/BP_PlayerController_Game.UpdateGameUI` _playercontroller)))

(fn `CreateWidgetsForPlayers`
  (bind _gamestate (message `/Game/_Main/Blueprints/Interfaces/BPI_GameState.GetGameState` (`GameplayStatics.GetGameState`)))
  (bind _players (`/Game/_Main/Framework/BP_GameStateBase_Game.Players` _gamestate))
  (bind _keys (`BlueprintMapLibrary.Map_Keys` _players))
  (for _array_element _keys
    (bind _playercontroller (message `/Game/_Main/Blueprints/Interfaces/BPI_CharacterController.GetPlayerController` (`PlayerState.GetPlayerController` (`GameplayStatics.GetPlayerStateFromUniqueNetId` (`.PlayerUniqueId_13_A48F12A04FD4F1A5D458D2B63D7A2242` (break `/Game/_Main/Blueprints/Structures/S_PlayerInfo` (`BlueprintMapLibrary.Map_Find` _players _array_element)))))))
    (`/Game/_Main/Framework/BP_PlayerController_Game.CreateLocalTurnlUI` _playercontroller)
    (`/Game/_Main/Framework/BP_PlayerController_Game.CreateLocalGameUI` _playercontroller)
    (`/Game/_Main/Framework/BP_PlayerController_Game.CreateMatchUI` _playercontroller)))

(fn `GetGameMode`
  (returns (Gamemode :type "/Game/_Main/Framework/BP_GameModeBase_Game Object Reference"))
  (return self))

(fn `Select Next Color`
  (returns (NextColor :type "/Game/_Main/Blueprints/Enums/E_Color Enum"))
  (locals (LocalPlayers :type "Map of /Game/_Main/Blueprints/Enums/E_Color Enum to /Game/_Main/Blueprints/Structures/S_PlayerInfo Structure") (LocalNextTurn :type Integer) (LocalPlayersKeys :type "Array of Integer") (LocalMaxColors :type Integer :default 4) (NextColorIsFound :type Boolean :default true))
  (bind _gamestate (message `/Game/_Main/Blueprints/Interfaces/BPI_GameState.GetGameState` (`GameplayStatics.GetGameState`)))
  (bind _result (`/Engine/EditorBlueprintResources/StandardMacros.IncrementInt` (`KismetMathLibrary.Conv_ByteToInt` (`/Game/_Main/Framework/BP_GameStateBase_Game.CurrentTurn` _gamestate)))
    (:`  `
      (set `local.LocalNextTurn` _result)
      ;[1 1 1] Add Players colors to the integer array
      (bind _keys (`BlueprintMapLibrary.Map_Keys` (`/Game/_Main/Framework/BP_GameStateBase_Game.Players` _gamestate)))
      (for _array_element _keys
        (`KismetArrayLibrary.Array_Add` (`local.LocalPlayersKeys`) (`KismetMathLibrary.Conv_ByteToInt` _array_element)))
      (while (`local.NextColorIsFound`)
        ;[1 1 1] Check if one of the players have Next Color Id
        (if (`KismetArrayLibrary.Array_Contains` (`local.LocalPlayersKeys`) (`local.LocalNextTurn`))
          ;[1 1 1] Exit While loop if next player is found
          (set `local.NextColorIsFound` false)
          (else
            ;[1 1 1] Increment Next Player Color if current Next Color is not found
            (bind _result_2 (`/Engine/EditorBlueprintResources/StandardMacros.IncrementInt` (`local.LocalNextTurn`))
              (:`  `
                (if (>= _result_2 (`local.LocalMaxColors`))
                  (set `local.LocalNextTurn` 0)))))))
      ;[1 1 1] Return next player color
      (return (cast `/Game/_Main/Blueprints/Enums/E_Color` (`KismetMathLibrary.Conv_IntToByte` (`local.LocalNextTurn`)))))))

(fn `ShowNextPlayerUI`
  (params (UniqueId :type "UniqueNetIdRepl Structure (by ref)"))
  (bind _playerstate (message `/Game/_Main/Blueprints/Interfaces/BPI_PlayerState.GetPlayerState` (`GameplayStatics.GetPlayerStateFromUniqueNetId` UniqueId)))
  (bind _playercontroller (message `/Game/_Main/Blueprints/Interfaces/BPI_CharacterController.GetPlayerController` (`PlayerState.GetPlayerController` _playerstate)))
  (`/Game/_Main/Framework/BP_PlayerController_Game.ShowTurnUi` _playercontroller))

(fn `UpdatePlayersForWidget`
  (bind _gamestate (message `/Game/_Main/Blueprints/Interfaces/BPI_GameState.GetGameState` (`GameplayStatics.GetGameState`)))
  (bind _widgetdata2 (`/Game/_Main/Framework/BP_GameStateBase_Game.WidgetData2` _gamestate))
  (for (_array_element _array_index) _widgetdata2
    (bind (_playerid _playeruniqueid _currentturn _color) (break `/Game/_Main/Blueprints/Structures/S_AllPlayerInfo` _array_element))
    (bind _value (`BlueprintMapLibrary.Map_Find` (`/Game/_Main/Framework/BP_GameStateBase_Game.Players` _gamestate) _color))
    (`KismetArrayLibrary.Array_Set` _widgetdata2 _array_index (make `/Game/_Main/Blueprints/Structures/S_AllPlayerInfo` (break `/Game/_Main/Blueprints/Structures/S_PlayerInfo` _value) (`.PlayerUniqueId_13_A48F12A04FD4F1A5D458D2B63D7A2242` (break `/Game/_Main/Blueprints/Structures/S_PlayerInfo` _value)) (`.CurrentTurn_6_69458CBC41FBB48FD41A2EA1BC060997` (break `/Game/_Main/Blueprints/Structures/S_PlayerInfo` _value)) _color))))

(fn `UpdatePlayerTurn`
  (params (NextColor :type "/Game/_Main/Blueprints/Enums/E_Color Enum" :default "NewEnumerator4"))
  (returns (PlayerID :type "UniqueNetIdRepl Structure"))
  (locals (LocalNextColor :type "/Game/_Main/Blueprints/Enums/E_Color Enum" :default "NewEnumerator4"))
  (set `local.LocalNextColor` NextColor)
  (bind _gamestate (message `/Game/_Main/Blueprints/Interfaces/BPI_GameState.GetGameState` (`GameplayStatics.GetGameState`)))
  (bind _currentturn (`/Game/_Main/Framework/BP_GameStateBase_Game.CurrentTurn` _gamestate))
  (if (not (`|EnumEquality` _currentturn "NewEnumerator4"))
    (bind _players (`/Game/_Main/Framework/BP_GameStateBase_Game.Players` _gamestate))
    (bind _value (`BlueprintMapLibrary.Map_Find` _players _currentturn))
    (`BlueprintMapLibrary.Map_Add` _players _currentturn (make `/Game/_Main/Blueprints/Structures/S_PlayerInfo` (break `/Game/_Main/Blueprints/Structures/S_PlayerInfo` _value) (`.PlayerUniqueId_13_A48F12A04FD4F1A5D458D2B63D7A2242` (break `/Game/_Main/Blueprints/Structures/S_PlayerInfo` _value)))))
  (bind _players_2 (`/Game/_Main/Framework/BP_GameStateBase_Game.Players` _gamestate))
  (bind _value_2 (`BlueprintMapLibrary.Map_Find` _players_2 (`local.LocalNextColor`)))
  (`BlueprintMapLibrary.Map_Add` _players_2 (`local.LocalNextColor`) (make `/Game/_Main/Blueprints/Structures/S_PlayerInfo` (break `/Game/_Main/Blueprints/Structures/S_PlayerInfo` _value_2) (`.PlayerUniqueId_13_A48F12A04FD4F1A5D458D2B63D7A2242` (break `/Game/_Main/Blueprints/Structures/S_PlayerInfo` _value_2)) true))
  (bind _gamestate_2 (message `/Game/_Main/Blueprints/Interfaces/BPI_GameState.GetGameState` (`GameplayStatics.GetGameState`)))
  (`self.UpdatePlayersForWidget`)
  (set `/Game/_Main/Framework/BP_GameStateBase_Game.CurrentTurn` (`local.LocalNextColor`) _gamestate_2)
  (return (`.PlayerUniqueId_13_A48F12A04FD4F1A5D458D2B63D7A2242` (break `/Game/_Main/Blueprints/Structures/S_PlayerInfo` _value_2))))

(fn `UserConstructionScript`)
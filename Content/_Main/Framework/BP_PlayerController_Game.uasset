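; BP_PlayerController_Game is the in-game player controller that sets up input and drives the players list on the HUD.
; On BeginPlay it sets game-only input, caches the BP_HUD_Game, adds the IMC_Game Enhanced Input mapping context and shows the mouse cursor.
; Holding the IA_PlayersList action shows the players list through the HUD, and releasing it closes the list.
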(event `self.ReceiveBeginPlay`
  ;[1 1 1] Initial setup of the Player Controller
  (`WidgetBlueprintLibrary.SetInputMode_GameOnly` self)
  (bind _asbp_hud_game (cast `/Game/_Main/Widgets/BP_HUD_Game` (`self.GetHUD`)))
  (set `self.My_HUD` _asbp_hud_game)
  (`EnhancedInputSubsystemInterface.AddMappingContext` (subsystem `EnhancedInputLocalPlayerSubsystem`) "/Game/_Main/Input/IMC_Game.IMC_Game" 0 (struct))
  (set `self.bShowMouseCursor` true))

(event `EnhancedInput|/Game/_Main/Input/Actions/IA_PlayersList`
  (params (ActionValue :type Boolean) (ElapsedSeconds :type "Float (double-precision)") (TriggeredSeconds :type "Float (double-precision)") (InputAction :type "InputAction Object Reference" :default "/Game/_Main/Input/Actions/IA_PlayersList.IA_PlayersList"))
  ;[1 1 1] Open List of Players
  (:`Started`
    (`/Game/_Main/Widgets/BP_HUD_Game.ShowPlayersList` (`self.My_HUD`)))
  (:`Completed`
    (`/Game/_Main/Widgets/BP_HUD_Game.ClosePlayersList` (`self.My_HUD`))))

(fn `UserConstructionScript`)
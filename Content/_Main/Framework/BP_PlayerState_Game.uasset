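; BP_PlayerState_Game is the game's player state, holding each player's name.
; On BeginPlay, the locally controlled player loads the "PlayerInfo" save slot as BP_MainSaveGame and passes its PlayerName to SendPlayerNameToServer.
; That event, intended to run on the server, stores the value in LocalPlayerName.
; A GetPlayerState function returns the state itself.
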(event `self.ReceiveBeginPlay`
  (bind _returnvalue (`self.GetPlayerController`))
  ;[1 1 1] Load Player Name from the Safe file and send it to the server
  (`/Engine/EditorBlueprintResources/StandardMacros.IsValid` _returnvalue
    (:`Is Valid`
      (if (`Controller.IsLocalController` _returnvalue)
        (bind _returnvalue_2 (`GameplayStatics.LoadGameFromSlot` "PlayerInfo"))
        (bind _asbp_main_save_game (cast `/Game/_Main/Framework/BP_MainSaveGame` _returnvalue_2))
        (`self.SendPlayerNameToServer` (`/Game/_Main/Framework/BP_MainSaveGame.PlayerName` _asbp_main_save_game))))))

(event `SendPlayerNameToServer`
  (params (PlayerName :type Text))
  ;[1 1 1] Send player name on the Server
  (set `self.LocalPlayerName` PlayerName))

(fn `GetPlayerState`
  (returns (PlayerState :type "/Game/_Main/Framework/BP_PlayerState_Game Object Reference"))
  (return self))

(fn `UserConstructionScript`)
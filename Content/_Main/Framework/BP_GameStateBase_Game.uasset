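; BP_GameStateBase_Game is a game state that indexes the board cells placed in the level.
; On BeginPlay it gathers every BP_CellBoard into the Cells array and maps each one by its Index in CellsMap.
; It does the same for BP_CellFinish actors, keying them by Index in CellsFinishMap for lookup.
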(event `self.ReceiveBeginPlay`
  (bind _outactors (`GameplayStatics.GetAllActorsOfClass` "/Game/_Main/BoardItems/Cells/BP_CellBoard.BP_CellBoard_C"))
  (set `self.Cells` _outactors)
  (for _array_element (`self.Cells`)
    (`BlueprintMapLibrary.Map_Add` (`self.CellsMap`) (`/Game/_Main/BoardItems/Cells/BP_Cell.Index` _array_element) _array_element))
  (bind _outactors_2 (`GameplayStatics.GetAllActorsOfClass` "/Game/_Main/BoardItems/Cells/BP_CellFinish.BP_CellFinish_C"))
  (for _array_element_2 _outactors_2
    (`BlueprintMapLibrary.Map_Add` (`self.CellsFinishMap`) (`/Game/_Main/BoardItems/Cells/BP_Cell.Index` _array_element_2) _array_element_2)))

(fn `UserConstructionScript`)
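; BP_CellStart is a start cell among the board items that creates a figurine at its own position.
; CreateFigurineServer spawns a BP_Figurine at the cell's transform, sets that figurine's CurrentCell to this cell and stores it as CurrentFigurine, linking the two both ways.
; BeginPlay and the construction script only call their parents, and nothing in this file calls the spawn event.
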(event `self.ReceiveBeginPlay`
  (`parent.ReceiveBeginPlay`))

(event `CreateFigurineServer`
  (bind _returnvalue (`|SpawnActorFromClass` "/Game/_Main/BoardItems/BP_Figurine.BP_Figurine_C" (`self.GetTransform`) "Undefined" "MultiplyWithRoot" null null))
  (set `/Game/_Main/BoardItems/BP_Figurine.CurrentCell` self _returnvalue)
  (set `self.CurrentFigurine` _returnvalue))

(fn `UserConstructionScript`
  (`parent.UserConstructionScript`))
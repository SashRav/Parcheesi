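; BP_CellBoard is a board cell that tracks a current and second figurine for captures and two-figurine "gates".
; Events forward to Multicast counterparts; working logic clears gate status and promotes the second figurine to current.
; Capturing calls helpers to send the occupant to start and move in the newcomer, branching on its status.
; Both helpers and gate construction are currently empty, their logic left in unconnected nodes.
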(event `DestroyGates`
  ;[1 1 1] Destroying Gates
  (`self.DestroyGatesMulticast`))

(event `MoveSecondToCurrent`
  ;[1 1 1] Destroying Gates
  (`self.MoveSecondToCurrentMulticast`))

(event `MoveSecondToCurrentMulticast`
  ;[1 1 1] Destroying Gates
  (set `self.CurrentFigurine` (`self.SecondFigurine`))
  (set `self.SecondFigurine` null)
  (`self.K2_SetActorLocation` (`self.CurrentFigurine`) (`self.K2_GetActorLocation`) false false))

(event `DestroyGatesMulticast`
  ;[1 1 1] Destroying Gates
  (set `self.HasGates` false)
  (bind _secondfigurine (`self.SecondFigurine`)
    (:`then`
      (set `/Game/_Main/Blueprints/BoardItems/BP_Figurine.GatesStatus` "NewEnumerator0" _secondfigurine))
    (:`else`
      _))
  (bind _currentfigurine (`self.CurrentFigurine`)
    (:`then`
      (set `/Game/_Main/Blueprints/BoardItems/BP_Figurine.GatesStatus` "NewEnumerator0" _currentfigurine))
    (:`else`)))

(event `ConstructGates`
  (params (NewFigurine :type "/Game/_Main/Blueprints/BoardItems/BP_Figurine Object Reference"))
  ;[1 1 1] Gates Constructing
  (`self.ConstructGatesMulticast` NewFigurine))

(event `ConstructGatesMulticast`
  (params (NewFigurine :type "/Game/_Main/Blueprints/BoardItems/BP_Figurine Object Reference"))
  ;[1 1 1] Gates Constructing
)

(event `DriveCurrentFigurineFromCell`
  (params (NewFigurine :type "/Game/_Main/Blueprints/BoardItems/BP_Figurine Object Reference"))
  ;[1 1 1] Overlapping enemy figurine
  (`self.DriveCurrentFigurineFromCellMulticast` NewFigurine))

(event `DriveCurrentFigurineFromCellMulticast`
  (params (NewFigurine :type "/Game/_Main/Blueprints/BoardItems/BP_Figurine Object Reference"))
  ;[1 1 1] Overlapping enemy figurine
  (`self.MoveCurrentFigurineToStart`)
  (switch `/Game/_Main/Blueprints/Enums/E_FigurineStatus` (`/Game/_Main/Blueprints/BoardItems/BP_Figurine.FigurineStatus` NewFigurine)
    (:`NewEnumerator0`
      (`self.MoveNewFigurine` NewFigurine true))
    (:`NewEnumerator1`
      (`self.MoveNewFigurine` NewFigurine))))

(fn `MoveCurrentFigurineToStart`
  (locals (LocalStartCell :type "/Game/_Main/Blueprints/BoardItems/Cells/BP_CellStart Object Reference")))

(fn `MoveNewFigurine`
  (params (`New Figurine` :type "/Game/_Main/Blueprints/BoardItems/BP_Figurine Object Reference") (IsMovingOnBoard :type Boolean))
  (locals (LocalNewFigurine :type "/Game/_Main/Blueprints/BoardItems/BP_Figurine Object Reference")))

(fn `UserConstructionScript`
  (`parent.UserConstructionScript`))
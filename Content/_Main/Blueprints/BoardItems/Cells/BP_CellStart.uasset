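; BP_CellStart is a board-game start cell that spawns a player's figurine.
; On BeginPlay it adds the player start tag from GameStart to its own actor tags.
; CreateFigurineServer spawns a BP_Figurine at the cell's transform, passing itself, the finish cell, the closest board cell's index and the owner tag, then stores the figurine reference.
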(event `self.ReceiveBeginPlay`
  ;[1 1 1] Add start tag to the current Start cell tags
  (`parent.ReceiveBeginPlay`)
  (`KismetArrayLibrary.Array_Add` (`self.Tags`) (`PlayerStart.PlayerStartTag` (`self.GameStart`))))

(event `CreateFigurineServer`
  ;[1 1 1] Create Figurine on the cell
  (set `self.BoardFirstCellID` (`/Game/_Main/Blueprints/BoardItems/Cells/BP_Cell.Index` (`self.ClosestBoardCell`)))
  (bind _returnvalue (`|SpawnActorFromClass` "/Game/_Main/Blueprints/BoardItems/BP_Figurine.BP_Figurine_C" (`self.GetTransform`) "Undefined" "MultiplyWithRoot" null (`self.FinishCell`) (`self.BoardFirstCellID`) self (`PlayerStart.PlayerStartTag` (`self.GameStart`)) null))
  (set `self.CreatedFigurine` _returnvalue))

(fn `UserConstructionScript`
  (`parent.UserConstructionScript`))
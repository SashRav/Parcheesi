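; BP_Figurine is a player's board-game pawn that takes its start cell's material, supports highlighted selection and moves between cells.
; Moves rebuild a spline through game-state board or finish cell locations, then a timeline slides the mesh along it.
; When a second-gates move ends, two figurines sharing a cell are offset to opposite sides, based on the previous cell's alignment.
; Returning to start resets cell index and status, animates back and plays a kick sound.
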(event `self.ReceiveBeginPlay`
  ;[1 1 1] Figurine initial Setup
  (`PrimitiveComponent.SetMaterial` (`self.StaticMesh`) 0 (`PrimitiveComponent.GetMaterial` (`/Game/_Main/Blueprints/BoardItems/Cells/BP_Cell.Cylinder` (`self.StartCell`)) 0))
  (`KismetArrayLibrary.Array_Add` (`self.Tags`) (`self.PlayerOwnerTag`)))

(event `SelectFigurineMulticast`
  (bind _staticmesh (`self.StaticMesh`))
  ;[1 1 1] Selecting figurine
  (`CCCSelectItem.SelectThisItem` (`self.CCCSelectItem`) "/Game/_Main/VFX/NS_SelectedFigurine.NS_SelectedFigurine" _staticmesh _staticmesh "/Game/_Main/Materials/Overlay/M_Overlay.M_Overlay"))

(event `MoveFigurineToNextPoint`
  (params (IsSelectedFigurineSecondGates :type Boolean) (CellsOnPath :type "Array of Integer"))
  ;[1 1 1] Figurine movement
  ;;[0.5212 1 0.4969] Movement between cells
  (`self.MoveFigurineToPoint` IsSelectedFigurineSecondGates CellsOnPath))

(event `UpdateGatesFigurinesOnServer`
  ;[1 1 1] Figurine movement
  ;;[0.5212 1 0.4969] Movement between cells
  (`self.UpdateGatesFigurines`))

(event `DeselectFigurineMulticast`
  ;[1 1 1] Selecting figurine
  (`CCCSelectItem.DeselectThisItem` (`self.CCCSelectItem`) (`self.StaticMesh`)))

(event `MoveFigurineToStart`
  ;[1 1 1] Figurine movement
  ;;[0.7427 1 0.7503] Moving figurine back to start cell
  (set `self.CurrentCellIndex` 0)
  (set `self.FigurineStatus` "NewEnumerator0")
  (`self.MoveFigurineToStartVisualMulticast`))

(event `MoveFigurineToStartVisualMulticast`
  ;[1 1 1] Figurine movement
  ;;[0.7427 1 0.7503] Moving figurine back to start cell
  (`self.MoveFigurineFromBoardToStart`)
  (`GameplayStatics.PlaySound2D` "/Game/_Main/Sound/W_Kick.W_Kick" 1.0 1.0 0.0 null null))

(event `MoveBySpline`
  (params (IsMovingToSecondGates :type Boolean))
  ;[1 1 1] Figurine movement
  ;;[0.6487 1 0.6273] Moving animation
  (bind (_direction _newtrack_0) (`Timeline|Timeline` :!via `PlayFromStart`)
    (:`Update`
      (`SceneComponent.K2_SetWorldLocation` (`self.StaticMesh`) (`SplineComponent.GetLocationAtTime` (`self.Spline`) _newtrack_0 "World" false) false false))
    (:`Finished`
      (if IsMovingToSecondGates
        (`self.UpdateGatesFigurinesOnServer`)))))

(fn `MoveFigurineFromBoardToStart`
  (bind _spline (`self.Spline`))
  (`SplineComponent.ClearSplinePoints` _spline true)
  (`SplineComponent.AddSplinePoint` _spline (`SceneComponent.K2_GetComponentLocation` (`self.StaticMesh`)) "World" true)
  (`SplineComponent.AddSplinePoint` (`self.Spline`) (`self.K2_GetActorLocation` (`self.StartCell`)) "World" true)
  (`self.MoveBySpline` false))

(fn `MoveFigurineToPoint`
  (params (IsSelectedFigurineSecondGates :type Boolean) (CellsOnPath :type "Array of Integer"))
  (locals (LocalTargetPoint :type "Vector Structure") (LocalCurrentWorldLocation :type "Vector Structure") (LocalCells :type "Array of Integer") (LocalIsSecondGates :type Boolean))
  (bind _spline (`self.Spline`))
  (set `local.LocalIsSecondGates` IsSelectedFigurineSecondGates)
  (bind _output_get (set `local.LocalCells` CellsOnPath))
  (if (not (`KismetArrayLibrary.Array_IsEmpty` _output_get))
    (`SplineComponent.ClearSplinePoints` _spline true)
    (`SplineComponent.AddSplinePoint` _spline (`SceneComponent.K2_GetComponentLocation` (`self.StaticMesh`)) "World" true)
    (for _array_element (`local.LocalCells`)
      (bind _gamestate (message `/Game/_Main/Blueprints/Interfaces/BPI_GameState.GetGameState` (`GameplayStatics.GetGameState`)))
      (bind (_value _returnvalue) (`BlueprintMapLibrary.Map_Find` (`/Game/_Main/Framework/BP_GameStateBase_Game.BoardCells` _gamestate) _array_element))
      (if _returnvalue
        (`SplineComponent.AddSplinePoint` (`self.Spline`) (`self.K2_GetActorLocation` (break `/Game/_Main/Blueprints/Structures/S_BoardCellInfo` _value)) "World" true)
        (else
          (`SplineComponent.AddSplinePoint` (`self.Spline`) (`self.K2_GetActorLocation` (break `/Game/_Main/Blueprints/Structures/S_FinishCellInfo` (`BlueprintMapLibrary.Map_Find` (`/Game/_Main/Framework/BP_GameStateBase_Game.FinishCells` _gamestate) _array_element))) "World" true))))
    (`self.MoveBySpline` (`local.LocalIsSecondGates`))
    (else
      (`KismetSystemLibrary.PrintString` "Cells on path array is Empty!"))))

(fn `UpdateGatesFigurines`
  (locals (LocalCurrentCellLocation :type "Vector Structure") (LocalPrevCellLocation :type "Vector Structure"))
  (bind (_localprevcelllocation_x _localprevcelllocation_y) (`KismetMathLibrary.BreakVector` (`local.LocalPrevCellLocation`)))
  (bind (_localcurrentcelllocation_x _localcurrentcelllocation_y) (`KismetMathLibrary.BreakVector` (`local.LocalCurrentCellLocation`)))
  (bind _localprevcelllocation_x_2 (`KismetMathLibrary.BreakVector` (`local.LocalPrevCellLocation`)))
  (bind _localcurrentcelllocation_x_2 (`KismetMathLibrary.BreakVector` (`local.LocalCurrentCellLocation`)))
  (bind _returnvalue (- (`self.CurrentCellIndex`) 1))
  (bind _gamestate (message `/Game/_Main/Blueprints/Interfaces/BPI_GameState.GetGameState` (`GameplayStatics.GetGameState`)))
  (bind _value (`BlueprintMapLibrary.Map_Find` (`/Game/_Main/Framework/BP_GameStateBase_Game.BoardCells` _gamestate) (`self.CurrentCellIndex`)))
  (if (and (`KismetSystemLibrary.IsValid` (`.FirstCurrentFigurine_12_FDEFEAB24A7C52C2E032699425ABB1CF` (break `/Game/_Main/Blueprints/Structures/S_BoardCellInfo` _value))) (`KismetSystemLibrary.IsValid` (`.SecondCurrentFigurine_13_31A29C344A72514920C6E5B5A91D3A85` (break `/Game/_Main/Blueprints/Structures/S_BoardCellInfo` _value))))
    (`GameplayStatics.PlaySound2D` "/Game/_Main/Sound/W_Build.W_Build" 1.0 1.0 0.0 null null)
    (set `local.LocalCurrentCellLocation` (`self.K2_GetActorLocation` (break `/Game/_Main/Blueprints/Structures/S_BoardCellInfo` _value)))
    (bind _gamestate_2 (message `/Game/_Main/Blueprints/Interfaces/BPI_GameState.GetGameState` (`GameplayStatics.GetGameState`)))
    (if (>= _returnvalue 0)
      (set `local.LocalPrevCellLocation` (`self.K2_GetActorLocation` (break `/Game/_Main/Blueprints/Structures/S_BoardCellInfo` (`BlueprintMapLibrary.Map_Find` (`/Game/_Main/Framework/BP_GameStateBase_Game.BoardCells` _gamestate_2) _returnvalue))))
      (else
        (bind _boardcells (`/Game/_Main/Framework/BP_GameStateBase_Game.BoardCells` _gamestate_2))
        (set `local.LocalPrevCellLocation` (`self.K2_GetActorLocation` (break `/Game/_Main/Blueprints/Structures/S_BoardCellInfo` (`BlueprintMapLibrary.Map_Find` _boardcells (- (`BlueprintMapLibrary.Map_Length` _boardcells) 1)))))))
    (if (`KismetMathLibrary.NearlyEqual_FloatFloat` _localprevcelllocation_x_2 _localcurrentcelllocation_x_2 100.0)
      (bind _gamestate_3 (message `/Game/_Main/Blueprints/Interfaces/BPI_GameState.GetGameState` (`GameplayStatics.GetGameState`)))
      (bind _value_2 (`BlueprintMapLibrary.Map_Find` (`/Game/_Main/Framework/BP_GameStateBase_Game.BoardCells` _gamestate_3) (`self.CurrentCellIndex`)))
      (`self.K2_SetActorLocation` (`.FirstCurrentFigurine_12_FDEFEAB24A7C52C2E032699425ABB1CF` (break `/Game/_Main/Blueprints/Structures/S_BoardCellInfo` _value_2)) (+ (`self.K2_GetActorLocation` (`.FirstCurrentFigurine_12_FDEFEAB24A7C52C2E032699425ABB1CF` (break `/Game/_Main/Blueprints/Structures/S_BoardCellInfo` _value_2))) (100.0 0.0 0.0)) false false)
      (`self.K2_SetActorLocation` (`.SecondCurrentFigurine_13_31A29C344A72514920C6E5B5A91D3A85` (break `/Game/_Main/Blueprints/Structures/S_BoardCellInfo` _value_2)) (+ (`self.K2_GetActorLocation` (`.SecondCurrentFigurine_13_31A29C344A72514920C6E5B5A91D3A85` (break `/Game/_Main/Blueprints/Structures/S_BoardCellInfo` _value_2))) (-100.0 0.0 0.0)) false false)
      (elif (`KismetMathLibrary.NearlyEqual_FloatFloat` _localprevcelllocation_y _localcurrentcelllocation_y 100.0)
        (bind _gamestate_4 (message `/Game/_Main/Blueprints/Interfaces/BPI_GameState.GetGameState` (`GameplayStatics.GetGameState`)))
        (bind _value_3 (`BlueprintMapLibrary.Map_Find` (`/Game/_Main/Framework/BP_GameStateBase_Game.BoardCells` _gamestate_4) (`self.CurrentCellIndex`)))
        (`self.K2_SetActorLocation` (`.FirstCurrentFigurine_12_FDEFEAB24A7C52C2E032699425ABB1CF` (break `/Game/_Main/Blueprints/Structures/S_BoardCellInfo` _value_3)) (+ (`self.K2_GetActorLocation` (`.FirstCurrentFigurine_12_FDEFEAB24A7C52C2E032699425ABB1CF` (break `/Game/_Main/Blueprints/Structures/S_BoardCellInfo` _value_3))) (0.0 100.0 0.0)) false false)
        (`self.K2_SetActorLocation` (`.SecondCurrentFigurine_13_31A29C344A72514920C6E5B5A91D3A85` (break `/Game/_Main/Blueprints/Structures/S_BoardCellInfo` _value_3)) (+ (`self.K2_GetActorLocation` (`.SecondCurrentFigurine_13_31A29C344A72514920C6E5B5A91D3A85` (break `/Game/_Main/Blueprints/Structures/S_BoardCellInfo` _value_3))) (0.0 -100.0 0.0)) false false)
        (else
          (`KismetSystemLibrary.PrintString` "Error finiding prev cell!" true true (struct :`R` 1.0 :`G` 0.063568 :`A` 1.0) 20.0))))))

(fn `UserConstructionScript`
  (`PrimitiveComponent.SetMaterial` (`self.StaticMesh`) 0 "/Game/_Main/Materials/Pawns/MI_Pawn_Red.MI_Pawn_Red"))
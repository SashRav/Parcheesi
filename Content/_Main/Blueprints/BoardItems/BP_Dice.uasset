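; BP_Dice is a board-item die that can be selected and tracks which side faces up.
; Multicast events pass selection to BPCSelectingItem, supplying a Niagara effect and overlay material for the highlight.
; A handler bound at BeginPlay updates CurrentSide from the box component with the highest world Z, converting that component's object name to the side number.
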(event `DeselectDiceMulticast`
  ;[1 1 1] Selecting and Deselecting Dice
  (`/Game/_Main/Blueprints/Components/BPC_SelectingItem.DeselectItemMulticast` (`self.BPC_SelectingItem`) (`self.StaticMeshComponent`)))

(event `SelectDiceMulticast`
  (bind _staticmeshcomponent (`self.StaticMeshComponent`))
  ;[1 1 1] Selecting and Deselecting Dice
  (`/Game/_Main/Blueprints/Components/BPC_SelectingItem.SelectItemMulticast` (`self.BPC_SelectingItem`) "/Game/_Main/VFX/NS_SelectedDice.NS_SelectedDice" _staticmeshcomponent _staticmeshcomponent "/Game/_Main/Materials/Overlay/M_Overlay.M_Overlay"))

(event `self.ReceiveBeginPlay`
  ;[1 1 1] Get Highest dice side
  (add `self.UpdateDiceSide` (delegate `UpdateDiceSide_Event`)))

(event `UpdateDiceSide_Event`
  ;[1 1 1] Get Highest dice side
  (set `self.CurrentSide` (`self.GetHighestComponent`)))

(fn `GetHighestComponent`
  (returns (Side :type Integer))
  (locals (LocalHighestZ :type "Float (double-precision)" :default -1000.0) (LocalHighestIndex :type Integer))
  (for _array_element (`self.K2_GetComponentsByClass` "/Script/Engine.BoxComponent")
    (bind (_returnvalue_x _returnvalue_y _returnvalue_z) (`KismetMathLibrary.BreakVector` (`SceneComponent.K2_GetComponentLocation` _array_element)))
    (if (> _returnvalue_z (`local.LocalHighestZ`))
      (set `local.LocalHighestIndex` (`KismetStringLibrary.Conv_StringToInt` (`KismetSystemLibrary.GetObjectName` _array_element)))
      (set `local.LocalHighestZ` _returnvalue_z)))
  (return (`local.LocalHighestIndex`)))

(fn `UserConstructionScript`)
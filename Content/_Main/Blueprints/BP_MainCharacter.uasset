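; Player actor for a multiplayer Ludo-style board game, handling figurine setup, dice and movement.
; On BeginPlay it fixes the camera, creates figurines at overlapped start cells and saves them to PlayerState.
; The selected figurine moves by the dice value through server-to-multicast events, using GameState cell maps for the wrapping board and finish lane.
; Landing on an own figurine builds blocking gates; landing on another drives it off.
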(event `self.ReceiveBeginPlay`
  ;[1 1 1] Create Figurines on Server
  (`self.GetCellsServer`)
  (`SceneComponent.K2_SetWorldLocationAndRotation` (`self.Camera`) (-260.0 50.0 4500.0) (struct :`Pitch` -90.0 :`Yaw` -180.0) false false))

(event `GetCellsServer`
  ;[1 1 1] Create Figurines on Server
  (`KismetSystemLibrary.Delay` 1.0)
  (bind _output_get (set `self.SelectedActors` (`PrimitiveComponent.GetOverlappingActors` (`self.Box`) "/Game/_Main/Blueprints/BoardItems/Cells/BP_CellStart.BP_CellStart_C")))
  (for _array_element _output_get
    (bind _asbp_cell_start (cast `/Game/_Main/Blueprints/BoardItems/Cells/BP_CellStart` _array_element))
    (`/Game/_Main/Blueprints/BoardItems/Cells/BP_CellStart.CreateFigurineServer` _asbp_cell_start)
    (`self.AddLocalActorMulticast` (`/Game/_Main/Blueprints/BoardItems/Cells/BP_Cell.CurrentFigurine` _asbp_cell_start)))
  (`self.SaveFigurinesToPlayerState`)
  (`self.GetFinishCells` (`/Game/_Main/Blueprints/BoardItems/Cells/BP_Cell.Index` (`/Game/_Main/Blueprints/BoardItems/BP_Figurine.FinishCell` (`|GetArrayItem` (`self.LocalFigurines`))))))

(event `AddLocalActorMulticast`
  (params (ActorToAdd :type "/Game/_Main/Blueprints/BoardItems/BP_Figurine Object Reference"))
  ;[1 1 1] Add figurines to local player State
  (`KismetArrayLibrary.Array_Add` (`self.LocalFigurines`) ActorToAdd))

(event `SaveFigurinesToPlayerState`
  ;[1 1 1] Add figurines to local player State
  (bind _asbp_player_state_game (cast `/Game/_Main/Framework/BP_PlayerState_Game` (`self.PlayerState`)))
  (set `/Game/_Main/Framework/BP_PlayerState_Game.LocalOwningFigurines` (`self.LocalFigurines`) _asbp_player_state_game))

(event `Key|One`
  (params (Key :type "Key Structure"))
  ;[0.4323 0.08781 0.08781] Debug Inputs
  (:`Pressed`
    (bind _asbp_player_state_game (cast `/Game/_Main/Framework/BP_PlayerState_Game` (`self.PlayerState`)))
    (bind _selectedfigurine (`/Game/_Main/Framework/BP_PlayerState_Game.SelectedFigurine` _asbp_player_state_game)
      (:`then`
        (`self.MoveFigurineOnServer` _selectedfigurine 1))
      (:`else`))))

(event `MoveFigurineOnServer`
  (params (Figurine :type "/Game/_Main/Blueprints/BoardItems/BP_Figurine Object Reference") (CellsToMove :type Integer))
  ;[1 1 1] Moving selected figurine
  (`self.MoveFigurineOnMulticast` Figurine (`/Game/_Main/Blueprints/BoardItems/BP_Figurine.ClosestBoardCell` Figurine) CellsToMove))

(event `MoveFigurineOnMulticast`
  (params (Figurine :type "/Game/_Main/Blueprints/BoardItems/BP_Figurine Object Reference") (ClosestStartCell :type "/Game/_Main/Blueprints/BoardItems/Cells/BP_CellBoard Object Reference") (CellsToMove :type Integer))
  ;[1 1 1] Moving selected figurine
  (`self.Move Figurine` ClosestStartCell Figurine CellsToMove))

(event `StartFigurineMovement`
  ;[1 1 1] Event called from the widget to move selected figurine
  (if (> (`self.SelectedDiceSide`) 0)
    (bind _asbp_player_state_game (cast `/Game/_Main/Framework/BP_PlayerState_Game` (`self.PlayerState`)))
    (bind _selectedfigurine (`/Game/_Main/Framework/BP_PlayerState_Game.SelectedFigurine` _asbp_player_state_game)
      (:`then`
        (`self.MoveFigurineOnServer` _selectedfigurine (`self.SelectedDiceSide`)))
      (:`else`))))

(event `SpawnDiceServer`
  ;[1 1 1] Spawn Dice blueprint
  (`self.SpawnDiceMulticast`))

(event `SelectDiceSideServer`
  (params (Dice :type "/Game/_Main/Blueprints/BoardItems/BP_Dice Object Reference"))
  ;[1 1 1] Select Dice Side
  (bind _output_get (set `self.SelectedDiceSide` (`/Game/_Main/Blueprints/BoardItems/BP_Dice.CurrentSide` Dice)))
  (`KismetSystemLibrary.PrintString` (`KismetStringLibrary.Conv_IntToString` _output_get)))

(event `SpawnDiceMulticast`
  ;[1 1 1] Spawn Dice blueprint
  (`/Engine/EditorBlueprintResources/ActorMacros.Switch Has Authority`
    (:`Authority`
      (`|SpawnActorFromClass` "/Game/_Main/Blueprints/BoardItems/BP_Dice.BP_Dice_C" (`self.Spawn Transform`) "Undefined" "MultiplyWithRoot" null null))))

(fn `CheckCellsOnPath`
  (params (Figurine :type "/Game/_Main/Blueprints/BoardItems/BP_Figurine Object Reference") (CurrentCell :type Integer) (NextCell :type Integer))
  (returns (CanFigurineMove :type Boolean))
  (locals (LocalFigurine :type "/Game/_Main/Blueprints/BoardItems/BP_Figurine Object Reference") (LocalFirstNextCell :type Integer) (LocalNextCell :type Integer))
  (set `local.LocalFigurine` Figurine)
  (bind _result (`/Engine/EditorBlueprintResources/StandardMacros.IncrementInt` CurrentCell)
    (:`  `
      (set `local.LocalFirstNextCell` _result)
      (set `local.LocalNextCell` NextCell)
      (for _index (range (`local.LocalFirstNextCell`) (+ (`local.LocalNextCell`) 1))
        (if (== (`BlueprintMapLibrary.Map_Find` (`self.Cells Map`) _index) (`/Game/_Main/Blueprints/BoardItems/BP_Figurine.ClosestBoardCell` (`local.LocalFigurine`)))
          (return false)))
      (return true))))

(fn `CountDestinationCell`
  (params (TotalCellsCount :type Integer) (FigurineIndex :type Integer) (CellsToMove :type Integer))
  (returns (DestinationCellIndex :type Integer))
  (locals (LocalDestinationCellIndex :type Integer) (LocalTotalCellsCount :type Integer))
  (set `local.LocalTotalCellsCount` TotalCellsCount)
  (bind _output_get (set `local.LocalDestinationCellIndex` (+ FigurineIndex CellsToMove)))
  (if (>= _output_get (`local.LocalTotalCellsCount`))
    (bind _output_get_2 (set `local.LocalDestinationCellIndex` (- (`local.LocalDestinationCellIndex`) (`local.LocalTotalCellsCount`))))
    (return _output_get_2)
    (else
      (return (`local.LocalDestinationCellIndex`)))))

(fn `GetFinishCells`
  (params (FirstFinishCellIndex :type Integer) (LastFinishCellIndex :type Integer))
  (returns (FinishCells :type "Map of Integer to /Game/_Main/Blueprints/BoardItems/Cells/BP_CellFinish Object Reference"))
  (locals (LocalAllFinishCells :type "Map of Integer to /Game/_Main/Blueprints/BoardItems/Cells/BP_CellFinish Object Reference") (LocalFirstFinishCellIndex :type Integer) (LocalLastFinishCellIndex :type Integer :default 3))
  (set `local.LocalFirstFinishCellIndex` FirstFinishCellIndex)
  (set `local.LocalLastFinishCellIndex` LastFinishCellIndex)
  (bind _asbp_game_state_base_game (cast `/Game/_Main/Framework/BP_GameStateBase_Game` (`GameplayStatics.GetGameState`)))
  (set `local.LocalAllFinishCells` (`/Game/_Main/Framework/BP_GameStateBase_Game.CellsFinishMap` _asbp_game_state_base_game))
  (for _index (range (`local.LocalFirstFinishCellIndex`) (+ (`local.LocalLastFinishCellIndex`) 1))
    (bind (_value _returnvalue) (`BlueprintMapLibrary.Map_Find` (`local.LocalAllFinishCells`) _index))
    (if _returnvalue
      (`BlueprintMapLibrary.Map_Add` (`self.FinishCells`) _index _value)))
  (return (`self.FinishCells`)))

(fn `Move Figurine`
  (params (ClosetsStartCell :type "/Game/_Main/Blueprints/BoardItems/Cells/BP_CellBoard Object Reference") (Figurine :type "/Game/_Main/Blueprints/BoardItems/BP_Figurine Object Reference") (CellsToMove :type Integer))
  (locals (LocalCellsToMove :type Integer :default 1) (LocalFigurine :type "/Game/_Main/Blueprints/BoardItems/BP_Figurine Object Reference") (LocalClosestCell :type "/Game/_Main/Blueprints/BoardItems/Cells/BP_CellBoard Object Reference"))
  (bind _index (`/Game/_Main/Blueprints/BoardItems/Cells/BP_Cell.Index` (`/Game/_Main/Blueprints/BoardItems/BP_Figurine.FinishCell` (`local.LocalFigurine`))))
  (set `local.LocalClosestCell` ClosetsStartCell)
  (set `local.LocalFigurine` Figurine)
  (set `local.LocalCellsToMove` CellsToMove)
  (switch `/Game/_Main/Blueprints/Enums/E_GatesStatus` (`/Game/_Main/Blueprints/BoardItems/BP_Figurine.GatesStatus` (`local.LocalFigurine`))
    (:`NewEnumerator0`
      (switch `/Game/_Main/Blueprints/Enums/E_FigurineStatus` (`/Game/_Main/Blueprints/BoardItems/BP_Figurine.FigurineStatus` (`local.LocalFigurine`))
        (:`NewEnumerator0`
          (`self.MoveFigurineOnBoard` (`local.LocalFigurine`) (`local.LocalClosestCell`)))
        (:`NewEnumerator1`
          (bind _asbp_game_state_base_game (cast `/Game/_Main/Framework/BP_GameStateBase_Game` (`GameplayStatics.GetGameState`)))
          (bind _output_get (set `self.Cells Map` (`/Game/_Main/Framework/BP_GameStateBase_Game.CellsMap` _asbp_game_state_base_game)))
          (`self.MoveFigurineToNextCell` _output_get (`local.LocalFigurine`) (`local.LocalCellsToMove`)))
        (:`NewEnumerator2`
          (bind _finishcells (`self.GetFinishCells` _index (+ _index 3)))
          (`self.MoveFigurineOnFinish` _finishcells (`local.LocalFigurine`) (`local.LocalCellsToMove`)))))
    (:`NewEnumerator1`
      (`KismetSystemLibrary.PrintString` "First Figurine ")
      (bind _asbp_game_state_base_game_2 (cast `/Game/_Main/Framework/BP_GameStateBase_Game` (`GameplayStatics.GetGameState`)))
      (bind _output_get_2 (set `self.Cells Map` (`/Game/_Main/Framework/BP_GameStateBase_Game.CellsMap` _asbp_game_state_base_game_2)))
      (`self.MoveFigurineToNextCellFromFirstGates` _output_get_2 (`local.LocalFigurine`) (`local.LocalCellsToMove`)))
    (:`NewEnumerator2`
      (`KismetSystemLibrary.PrintString` "Second Figurine")
      (bind _asbp_game_state_base_game_3 (cast `/Game/_Main/Framework/BP_GameStateBase_Game` (`GameplayStatics.GetGameState`)))
      (bind _output_get_3 (set `self.Cells Map` (`/Game/_Main/Framework/BP_GameStateBase_Game.CellsMap` _asbp_game_state_base_game_3)))
      (`self.MoveFigurineToNextCellFromSecondGates` _output_get_3 (`local.LocalFigurine`) (`local.LocalCellsToMove`)))))

(fn `MoveFigurineOnBoard`
  (params (Figurine :type "/Game/_Main/Blueprints/BoardItems/BP_Figurine Object Reference") (ClosestStartCell :type "/Game/_Main/Blueprints/BoardItems/Cells/BP_CellBoard Object Reference"))
  (locals (LocalFigurine :type "/Game/_Main/Blueprints/BoardItems/BP_Figurine Object Reference") (LocalClosestStartCell :type "/Game/_Main/Blueprints/BoardItems/Cells/BP_CellBoard Object Reference"))
  (set `local.LocalFigurine` Figurine)
  (set `local.LocalClosestStartCell` ClosestStartCell)
  (`/Game/_Main/Blueprints/BoardItems/Cells/BP_Cell.CurrentFigurine` (`local.LocalClosestStartCell`)
    (:`then`
      (`self.OverlapFigurinesOnCell` (`local.LocalFigurine`) (`local.LocalClosestStartCell`)))
    (:`else`
      (set `/Game/_Main/Blueprints/BoardItems/BP_Figurine.CurrentCell` (`local.LocalClosestStartCell`) (`local.LocalFigurine`))
      (set `/Game/_Main/Blueprints/BoardItems/BP_Figurine.CurrentIndex` (`/Game/_Main/Blueprints/BoardItems/Cells/BP_Cell.Index` (`local.LocalClosestStartCell`)) (`local.LocalFigurine`))
      (set `/Game/_Main/Blueprints/BoardItems/BP_Figurine.FigurineStatus` "NewEnumerator1" (`local.LocalFigurine`))
      (set `/Game/_Main/Blueprints/BoardItems/Cells/BP_Cell.CurrentFigurine` (`local.LocalFigurine`) (`local.LocalClosestStartCell`))
      (`self.K2_SetActorLocation` (`local.LocalFigurine`) (`self.K2_GetActorLocation` (`local.LocalClosestStartCell`)) false false))))

(fn `MoveFigurineOnFinish`
  (params (FinishCells :type "Map of Integer to /Game/_Main/Blueprints/BoardItems/Cells/BP_CellFinish Object Reference") (Figurine :type "/Game/_Main/Blueprints/BoardItems/BP_Figurine Object Reference") (CellsToMove :type Integer))
  (locals (LocalFinishCells :type "Map of Integer to /Game/_Main/Blueprints/BoardItems/Cells/BP_CellFinish Object Reference") (LocalFigurine :type "/Game/_Main/Blueprints/BoardItems/BP_Figurine Object Reference") (LocalCellsToMove :type Integer) (LocalNextCell :type "/Game/_Main/Blueprints/BoardItems/Cells/BP_CellFinish Object Reference"))
  (bind (_value _returnvalue) (`BlueprintMapLibrary.Map_Find` (`local.LocalFinishCells`) (+ (`/Game/_Main/Blueprints/BoardItems/BP_Figurine.CurrentIndex` (`local.LocalFigurine`)) (`local.LocalCellsToMove`))))
  (set `local.LocalFinishCells` FinishCells)
  (set `local.LocalFigurine` Figurine)
  (set `local.LocalCellsToMove` CellsToMove)
  (if _returnvalue
    (`KismetSystemLibrary.PrintString` "CanMoveOnFinish")
    (set `local.LocalNextCell` _value)
    (`/Game/_Main/Blueprints/BoardItems/Cells/BP_Cell.CurrentFigurine` (`local.LocalNextCell`)
      (:`then`
        (`KismetSystemLibrary.PrintString` "NextFinishCellIsNotEmpty"))
      (:`else`
        (set `/Game/_Main/Blueprints/BoardItems/Cells/BP_Cell.CurrentFigurine` null (`/Game/_Main/Blueprints/BoardItems/BP_Figurine.CurrentCell` (`local.LocalFigurine`)))
        (set `/Game/_Main/Blueprints/BoardItems/Cells/BP_Cell.CurrentFigurine` (`local.LocalFigurine`) (`local.LocalNextCell`))
        (set `/Game/_Main/Blueprints/BoardItems/BP_Figurine.CurrentCell` (`local.LocalNextCell`) (`local.LocalFigurine`))
        (set `/Game/_Main/Blueprints/BoardItems/BP_Figurine.CurrentIndex` (`/Game/_Main/Blueprints/BoardItems/Cells/BP_Cell.Index` (`local.LocalNextCell`)) (`local.LocalFigurine`))
        (`self.K2_SetActorLocation` (`local.LocalFigurine`) (`self.K2_GetActorLocation` (`local.LocalNextCell`)) false false)))
    (else
      (`KismetSystemLibrary.PrintString` "EndOfFinish"))))

(fn `MoveFigurineToNextCell`
  (params (CellsMap :type "Map of Integer to /Game/_Main/Blueprints/BoardItems/Cells/BP_CellBoard Object Reference") (Figurine :type "/Game/_Main/Blueprints/BoardItems/BP_Figurine Object Reference") (CellsToMove :type Integer))
  (locals (LocalFigurineIndex :type Integer :default 0) (LocalFigurine :type "/Game/_Main/Blueprints/BoardItems/BP_Figurine Object Reference") (LocalNextCellIndex :type Integer) (LocalCellsToMove :type Integer) (LocalNextCell :type "/Game/_Main/Blueprints/BoardItems/Cells/BP_CellBoard Object Reference") (LocalCellsCount :type Integer) (LocalCellsMap :type "Map of Integer to /Game/_Main/Blueprints/BoardItems/Cells/BP_CellBoard Object Reference"))
  (bind (_value _returnvalue) (`BlueprintMapLibrary.Map_Find` (`local.LocalCellsMap`) (`local.LocalNextCellIndex`)))
  (set `local.LocalCellsMap` CellsMap)
  (set `local.LocalFigurine` Figurine)
  (set `local.LocalCellsToMove` CellsToMove)
  (set `local.LocalCellsCount` (`BlueprintMapLibrary.Map_Length` (`local.LocalCellsMap`)))
  (set `local.LocalFigurineIndex` (`/Game/_Main/Blueprints/BoardItems/BP_Figurine.CurrentIndex` (`local.LocalFigurine`)))
  (bind _destinationcellindex (`self.CountDestinationCell` (`local.LocalCellsCount`) (`local.LocalFigurineIndex`) (`local.LocalCellsToMove`)))
  (set `local.LocalNextCellIndex` _destinationcellindex)
  (if (== (`local.LocalNextCellIndex`) (`/Game/_Main/Blueprints/BoardItems/BP_Figurine.ClosestBoardCellIndex` (`local.LocalFigurine`)))
    (`self.MoveToFinish` (`/Game/_Main/Blueprints/BoardItems/BP_Figurine.FinishCell` (`local.LocalFigurine`)) (`local.LocalFigurine`))
    (else
      (bind _canfigurinemove (`self.CheckCellsOnPath` (`local.LocalFigurine`) (`local.LocalFigurineIndex`) (`local.LocalNextCellIndex`)))
      (if _canfigurinemove
        (if _returnvalue
          (set `local.LocalNextCell` _value)
          (`/Game/_Main/Blueprints/BoardItems/Cells/BP_Cell.CurrentFigurine` (`local.LocalNextCell`)
            (:`then`
              (`self.OverlapFigurinesOnCell` (`local.LocalFigurine`) (`local.LocalNextCell`)))
            (:`else`
              (`KismetSystemLibrary.PrintString` "CanMove")
              (set `/Game/_Main/Blueprints/BoardItems/Cells/BP_Cell.CurrentFigurine` null (`/Game/_Main/Blueprints/BoardItems/BP_Figurine.CurrentCell` (`local.LocalFigurine`)))
              (set `/Game/_Main/Blueprints/BoardItems/Cells/BP_Cell.CurrentFigurine` (`local.LocalFigurine`) (`local.LocalNextCell`))
              (set `/Game/_Main/Blueprints/BoardItems/BP_Figurine.CurrentCell` (`local.LocalNextCell`) (`local.LocalFigurine`))
              (set `/Game/_Main/Blueprints/BoardItems/BP_Figurine.CurrentIndex` (`local.LocalNextCellIndex`) (`local.LocalFigurine`))
              (`self.K2_SetActorLocation` (`local.LocalFigurine`) (`self.K2_GetActorLocation` (`local.LocalNextCell`)) false false)))
          (else
            (`KismetSystemLibrary.PrintString` "Error. Target Cell did not find")))
        (else
          (`KismetSystemLibrary.PrintString` "Finish on the path"))))))

(fn `MoveFigurineToNextCellFromFirstGates`
  (params (CellsMap :type "Map of Integer to /Game/_Main/Blueprints/BoardItems/Cells/BP_CellBoard Object Reference") (Figurine :type "/Game/_Main/Blueprints/BoardItems/BP_Figurine Object Reference") (CellsToMove :type Integer))
  (locals (LocalFigurineIndex :type Integer :default 0) (LocalFigurine :type "/Game/_Main/Blueprints/BoardItems/BP_Figurine Object Reference") (LocalNextCellIndex :type Integer) (LocalCellsToMove :type Integer) (LocalNextCell :type "/Game/_Main/Blueprints/BoardItems/Cells/BP_CellBoard Object Reference") (LocalCellsCount :type Integer) (LocalCellsMap :type "Map of Integer to /Game/_Main/Blueprints/BoardItems/Cells/BP_CellBoard Object Reference"))
  (bind (_value _returnvalue) (`BlueprintMapLibrary.Map_Find` (`local.LocalCellsMap`) (`local.LocalNextCellIndex`)))
  (set `local.LocalCellsMap` CellsMap)
  (set `local.LocalFigurine` Figurine)
  (set `local.LocalCellsToMove` CellsToMove)
  (set `local.LocalCellsCount` (`BlueprintMapLibrary.Map_Length` (`local.LocalCellsMap`)))
  (set `local.LocalFigurineIndex` (`/Game/_Main/Blueprints/BoardItems/BP_Figurine.CurrentIndex` (`local.LocalFigurine`)))
  (bind _destinationcellindex (`self.CountDestinationCell` (`local.LocalCellsCount`) (`local.LocalFigurineIndex`) (`local.LocalCellsToMove`)))
  (set `local.LocalNextCellIndex` _destinationcellindex)
  (if (== (`local.LocalNextCellIndex`) (`/Game/_Main/Blueprints/BoardItems/BP_Figurine.ClosestBoardCellIndex` (`local.LocalFigurine`)))
    (`self.MoveToFinish` (`/Game/_Main/Blueprints/BoardItems/BP_Figurine.FinishCell` (`local.LocalFigurine`)) (`local.LocalFigurine`))
    (else
      (bind _canfigurinemove (`self.CheckCellsOnPath` (`local.LocalFigurine`) (`local.LocalFigurineIndex`) (`local.LocalNextCellIndex`)))
      (if _canfigurinemove
        (if _returnvalue
          (set `local.LocalNextCell` _value)
          (`/Game/_Main/Blueprints/BoardItems/Cells/BP_Cell.CurrentFigurine` (`local.LocalNextCell`)
            (:`then`
              (`self.OverlapFigurinesOnCell` (`local.LocalFigurine`) (`local.LocalNextCell`)))
            (:`else`
              (`KismetSystemLibrary.PrintString` "CanMove")
              (bind _asbp_cell_board (cast `/Game/_Main/Blueprints/BoardItems/Cells/BP_CellBoard` (`/Game/_Main/Blueprints/BoardItems/BP_Figurine.CurrentCell` (`local.LocalFigurine`))))
              (`/Game/_Main/Blueprints/BoardItems/Cells/BP_CellBoard.DestroyGates` _asbp_cell_board)
              (`/Game/_Main/Blueprints/BoardItems/Cells/BP_CellBoard.MoveSecondToCurrent` _asbp_cell_board)
              (set `/Game/_Main/Blueprints/BoardItems/Cells/BP_Cell.CurrentFigurine` (`local.LocalFigurine`) (`local.LocalNextCell`))
              (set `/Game/_Main/Blueprints/BoardItems/BP_Figurine.CurrentCell` (`local.LocalNextCell`) (`local.LocalFigurine`))
              (set `/Game/_Main/Blueprints/BoardItems/BP_Figurine.CurrentIndex` (`local.LocalNextCellIndex`) (`local.LocalFigurine`))
              (`self.K2_SetActorLocation` (`local.LocalFigurine`) (`self.K2_GetActorLocation` (`local.LocalNextCell`)) false false)))
          (else
            (`KismetSystemLibrary.PrintString` "Error. Target Cell did not find")))
        (else
          (`KismetSystemLibrary.PrintString` "Finish on the path"))))))

(fn `MoveFigurineToNextCellFromSecondGates`
  (params (CellsMap :type "Map of Integer to /Game/_Main/Blueprints/BoardItems/Cells/BP_CellBoard Object Reference") (Figurine :type "/Game/_Main/Blueprints/BoardItems/BP_Figurine Object Reference") (CellsToMove :type Integer))
  (locals (LocalFigurineIndex :type Integer :default 0) (LocalFigurine :type "/Game/_Main/Blueprints/BoardItems/BP_Figurine Object Reference") (LocalNextCellIndex :type Integer) (LocalCellsToMove :type Integer) (LocalNextCell :type "/Game/_Main/Blueprints/BoardItems/Cells/BP_CellBoard Object Reference") (LocalCellsCount :type Integer) (LocalCellsMap :type "Map of Integer to /Game/_Main/Blueprints/BoardItems/Cells/BP_CellBoard Object Reference"))
  (bind (_value _returnvalue) (`BlueprintMapLibrary.Map_Find` (`local.LocalCellsMap`) (`local.LocalNextCellIndex`)))
  (set `local.LocalCellsMap` CellsMap)
  (set `local.LocalFigurine` Figurine)
  (set `local.LocalCellsToMove` CellsToMove)
  (set `local.LocalCellsCount` (`BlueprintMapLibrary.Map_Length` (`local.LocalCellsMap`)))
  (set `local.LocalFigurineIndex` (`/Game/_Main/Blueprints/BoardItems/BP_Figurine.CurrentIndex` (`local.LocalFigurine`)))
  (bind _destinationcellindex (`self.CountDestinationCell` (`local.LocalCellsCount`) (`local.LocalFigurineIndex`) (`local.LocalCellsToMove`)))
  (set `local.LocalNextCellIndex` _destinationcellindex)
  (if (== (`local.LocalNextCellIndex`) (`/Game/_Main/Blueprints/BoardItems/BP_Figurine.ClosestBoardCellIndex` (`local.LocalFigurine`)))
    (`self.MoveToFinish` (`/Game/_Main/Blueprints/BoardItems/BP_Figurine.FinishCell` (`local.LocalFigurine`)) (`local.LocalFigurine`))
    (else
      (bind _canfigurinemove (`self.CheckCellsOnPath` (`local.LocalFigurine`) (`local.LocalFigurineIndex`) (`local.LocalNextCellIndex`)))
      (if _canfigurinemove
        (if _returnvalue
          (set `local.LocalNextCell` _value)
          (`/Game/_Main/Blueprints/BoardItems/Cells/BP_Cell.CurrentFigurine` (`local.LocalNextCell`)
            (:`then`
              (`self.OverlapFigurinesOnCell` (`local.LocalFigurine`) (`local.LocalNextCell`)))
            (:`else`
              (`KismetSystemLibrary.PrintString` "CanMove")
              (bind _asbp_cell_board (cast `/Game/_Main/Blueprints/BoardItems/Cells/BP_CellBoard` (`/Game/_Main/Blueprints/BoardItems/BP_Figurine.CurrentCell` (`local.LocalFigurine`))))
              (`/Game/_Main/Blueprints/BoardItems/Cells/BP_CellBoard.DestroyGates` _asbp_cell_board)
              (set `/Game/_Main/Blueprints/BoardItems/Cells/BP_CellBoard.SecondFigurine` null _asbp_cell_board)
              (set `/Game/_Main/Blueprints/BoardItems/Cells/BP_Cell.CurrentFigurine` (`local.LocalFigurine`) (`local.LocalNextCell`))
              (set `/Game/_Main/Blueprints/BoardItems/BP_Figurine.CurrentCell` (`local.LocalNextCell`) (`local.LocalFigurine`))
              (set `/Game/_Main/Blueprints/BoardItems/BP_Figurine.CurrentIndex` (`local.LocalNextCellIndex`) (`local.LocalFigurine`))
              (`self.K2_SetActorLocation` (`local.LocalFigurine`) (`self.K2_GetActorLocation` (`local.LocalNextCell`)) false false)))
          (else
            (`KismetSystemLibrary.PrintString` "Error. Target Cell did not find")))
        (else
          (`KismetSystemLibrary.PrintString` "Finish on the path"))))))

(fn `MoveToFinish`
  (params (FinishCell :type "/Game/_Main/Blueprints/BoardItems/Cells/BP_CellFinish Object Reference") (Figurine :type "/Game/_Main/Blueprints/BoardItems/BP_Figurine Object Reference"))
  (locals (LocalFigurine :type "/Game/_Main/Blueprints/BoardItems/BP_Figurine Object Reference") (LocalFinishCell :type "/Game/_Main/Blueprints/BoardItems/Cells/BP_CellFinish Object Reference"))
  (`/Game/_Main/Blueprints/BoardItems/Cells/BP_Cell.CurrentFigurine` FinishCell
    (:`then`
      (`KismetSystemLibrary.PrintString` "FirstFinishCellIsNotEmpt"))
    (:`else`
      (set `local.LocalFinishCell` FinishCell)
      (set `local.LocalFigurine` Figurine)
      (set `/Game/_Main/Blueprints/BoardItems/Cells/BP_Cell.CurrentFigurine` null (`/Game/_Main/Blueprints/BoardItems/BP_Figurine.CurrentCell` (`local.LocalFigurine`)))
      (set `/Game/_Main/Blueprints/BoardItems/Cells/BP_Cell.CurrentFigurine` (`local.LocalFigurine`) (`local.LocalFinishCell`))
      (set `/Game/_Main/Blueprints/BoardItems/BP_Figurine.CurrentCell` (`local.LocalFinishCell`) (`local.LocalFigurine`))
      (set `/Game/_Main/Blueprints/BoardItems/BP_Figurine.FigurineStatus` "NewEnumerator2" (`local.LocalFigurine`))
      (set `/Game/_Main/Blueprints/BoardItems/BP_Figurine.CurrentIndex` (`/Game/_Main/Blueprints/BoardItems/Cells/BP_Cell.Index` (`local.LocalFinishCell`)) (`local.LocalFigurine`))
      (`self.K2_SetActorLocation` (`local.LocalFigurine`) (`self.K2_GetActorLocation` (`local.LocalFinishCell`)) false false))))

(fn `OverlapFigurinesOnCell`
  (params (Figurine :type "/Game/_Main/Blueprints/BoardItems/BP_Figurine Object Reference") (TargetCell :type "/Game/_Main/Blueprints/BoardItems/Cells/BP_CellBoard Object Reference"))
  (locals (LocalTargetCell :type "/Game/_Main/Blueprints/BoardItems/Cells/BP_CellBoard Object Reference") (LocalFigurine :type "/Game/_Main/Blueprints/BoardItems/BP_Figurine Object Reference"))
  (set `local.LocalFigurine` Figurine)
  (set `local.LocalTargetCell` TargetCell)
  (if (`/Game/_Main/Blueprints/BoardItems/Cells/BP_CellBoard.HasGates` (`local.LocalTargetCell`))
    (`KismetSystemLibrary.PrintString` "Unablae To move - Cell has Gates")
    (else
      (for _array_element (`self.LocalFigurines`)
        (if (== _array_element (`/Game/_Main/Blueprints/BoardItems/Cells/BP_Cell.CurrentFigurine` (`local.LocalTargetCell`)))
          (`/Game/_Main/Blueprints/BoardItems/Cells/BP_CellBoard.ConstructGates` (`local.LocalTargetCell`) (`local.LocalFigurine`))
          (return)))
      (`/Game/_Main/Blueprints/BoardItems/Cells/BP_CellBoard.DriveCurrentFigurineFromCell` (`local.LocalTargetCell`) (`local.LocalFigurine`)))))

(fn `UserConstructionScript`)
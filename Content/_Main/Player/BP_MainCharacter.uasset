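; BP_MainCharacter is the player character that spawns the player's starting figurines and registers them in player state.
; One second after possession, it caches BP_PlayerState_Game and calls a creation chain whose event names suggest server-to-multicast routing.
; That chain finds cells overlapping its Box, has each BP_CellStart create a figurine, then stores the collected figurines as the state's LocalOwningFigurines.
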(event `GetPSClient`
  ;[1 1 1] Add statr cells to player state
  (bind _asbp_player_state_game (cast `/Game/_Main/Framework/BP_PlayerState_Game` (`self.PlayerState`)))
  (set `self.As BP Player State Game` _asbp_player_state_game)
  (`self.CreateFigurineServer`))

(event `self.ReceivePossessed`
  (params (NewController :type "Controller Object Reference"))
  ;[1 1 1] Add statr cells to player state
  (`KismetSystemLibrary.Delay` 1.0)
  (`self.GetPSClient`))

(event `CreateFigurineServer`
  ;[1 1 1] Create Figurine on the Start Cells
  (`self.CreateFigurineMult`))

(event `CreateFigurineMult`
  ;[1 1 1] Create Figurine on the Start Cells
  (for _array_element (`PrimitiveComponent.GetOverlappingActors` (`self.Box`) "/Game/_Main/BoardItems/Cells/BP_Cell.BP_Cell_C")
    (bind _asbp_cell_start (cast `/Game/_Main/BoardItems/Cells/BP_CellStart` _array_element))
    (`/Game/_Main/BoardItems/Cells/BP_CellStart.CreateFigurine` _asbp_cell_start)
    (`KismetArrayLibrary.Array_Add` (`self.SelectedFegurines`) (`/Game/_Main/BoardItems/Cells/BP_Cell.CurrentFigurine` _asbp_cell_start)))
  (`self.AddFigurinesToState`))

(event `AddFigurinesToState`
  ;[1 1 1] Add figurines to Player State
  (set `/Game/_Main/Framework/BP_PlayerState_Game.LocalOwningFigurines` (`self.SelectedFegurines`) (`self.As BP Player State Game`)))

(fn `UserConstructionScript`)